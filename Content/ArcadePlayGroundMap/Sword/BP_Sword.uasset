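; BP_Sword is a VR sword that motion controllers pick up and drop, and that cuts procedural meshes it touches.
; Pickup disables physics and attaches it to the given component at a fixed grip offset, while Drop detaches it and restores physics.
; A Plane component's overlap slices the mesh along that plane, capping the cut and simulating physics on the new half.
; A DoOnce, reset on end overlap, prevents repeated slices.
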(event `/Game/VirtualRealityBP/Blueprints/PickupActorInterface.Pickup`
  (params (AttachTo :type "SceneComponent Object Reference"))
  (`PrimitiveComponent.SetSimulatePhysics` (`self.StaticMeshComponent`) false)
  (`SceneComponent.K2_AttachToComponent` (`self.K2_GetRootComponent`) AttachTo "None" "SnapToTarget" "SnapToTarget" "KeepWorld" false)
  (`SceneComponent.K2_SetRelativeLocationAndRotation` (`self.StaticMeshComponent`) (3.76207 -2.53388 44.756413) (struct :`Pitch` -9.205244 :`Yaw` 0.484556 :`Roll` -93.026009) false false))

(event `/Game/VirtualRealityBP/Blueprints/PickupActorInterface.Drop`
  (`PrimitiveComponent.SetSimulatePhysics` (`self.StaticMeshComponent`) true)
  (`self.K2_DetachFromActor` "KeepWorld" "KeepWorld" "KeepWorld"))

(event `self.Plane.OnComponentBeginOverlap`
  (params (OverlappedComponent :type "PrimitiveComponent Object Reference") (OtherActor :type "Actor Object Reference") (OtherComp :type "PrimitiveComponent Object Reference") (OtherBodyIndex :type Integer) (bFromSweep :type Boolean) (SweepResult :type "HitResult Structure (by ref)"))
  (bind _plane (`self.Plane`))
  (`/Engine/EditorBlueprintResources/StandardMacros.DoOnce` false :!label _label
    (:`Completed`
      (bind _asprocedural_mesh_component (cast `ProceduralMeshComponent` OtherComp))
      (bind _outotherhalfprocmesh (`KismetProceduralMeshLibrary.SliceProceduralMesh` _asprocedural_mesh_component (`SceneComponent.K2_GetComponentLocation` _plane) (`SceneComponent.GetUpVector` _plane) true "CreateNewSectionForCap" "/Game/ArcadePlayGroundMap/Sword/AfterSlice.AfterSlice"))
      (`PrimitiveComponent.SetSimulatePhysics` _outotherhalfprocmesh true))))

(event `self.Plane.OnComponentEndOverlap`
  (params (OverlappedComponent :type "PrimitiveComponent Object Reference") (OtherActor :type "Actor Object Reference") (OtherComp :type "PrimitiveComponent Object Reference") (OtherBodyIndex :type Integer))
  (goto _label :!via `Reset`))

(fn `UserConstructionScript`)